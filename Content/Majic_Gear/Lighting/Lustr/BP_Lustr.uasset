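; BP_Lustr is a placeable Lustr lighting fixture with an arm, a light body and a rect light.
; The construction script applies rotation to the arm instance, and rotation plus tilt to the light instance and the rect light, so the emitter follows the body.
; Brightness and color variables set the rect light's intensity and color.
; All setup runs at construction; the event graph holds only disabled stubs.
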(event EventBeginPlay)

(event Collision|EventActorBeginOverlap
  (params (OtherActor :type Actor%20Object%20Reference)))

(event EventTick
  (params (DeltaSeconds :type Float%20%28single-precision%29)))

(fn ConstructionScript
  (bind _lustr_rotation (Variables|Default|GetLustr_Rotation))
  (bind _lustr_tilt (Variables|Default|GetLustr_Tilt))
  (bind _lustrrectlight (Variables|Default|GetLustrRectLight))
  (Components|InstancedStaticMesh|UpdateInstanceTransform (Variables|Default|GetArm) 0 (Math|Transform|MakeTransform "0, 0, 0" (Math|Rotator|MakeRotator 0.0 _lustr_rotation 0.0) "1.000000,1.000000,1.000000") false false false)
  (Components|InstancedStaticMesh|UpdateInstanceTransform (Variables|Default|GetLight) 0 (Math|Transform|MakeTransform "0.000000,20.000000,0.000000" (Math|Rotator|MakeRotator _lustr_rotation 0.0 _lustr_tilt) "1.000000,1.000000,1.000000") false false false)
  (Transformation|SetRelativeTransform _lustrrectlight (Math|Transform|MakeTransform "0, 0, 0" (Math|Rotator|MakeRotator 0.0 (* _lustr_rotation -1.0) (+ _lustr_tilt 9e+01)) "1.000000,1.000000,1.000000") true false)
  (Rendering|Components|Light|SetIntensity _lustrrectlight (Variables|Default|GetLustr_Brightness))
  (Rendering|Components|Light|SetLightColor _lustrrectlight (Variables|Default|GetLustr_Color) true))