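; BP_Skybox is a lighting fixture built from an instanced SkyBox mesh, two instanced legs and a rect light.
; The construction script adds the mesh instances, angles the box and light by SkyBoxAngle, and applies Brightness and SkyboxColor to the light.
; Tick adds SkyBoxAngle every frame as box roll and light yaw, so a non-zero angle spins them continuously, and reapplies Brightness.
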(event EventBeginPlay)

(event Collision|EventActorBeginOverlap
  (params (OtherActor :type Actor%20Object%20Reference)))

(event EventTick
  (params (DeltaSeconds :type Float%20%28single-precision%29))
  (bind _skyboxangle (Variables|Default|GetSkyBoxAngle))
  (Transformation|AddLocalRotation (Variables|Default|GetSkyBox) (Math|Rotator|MakeRotator _skyboxangle 0.0 0.0) false false)
  (Transformation|AddLocalRotation (Variables|Default|GetRectLight) (Math|Rotator|MakeRotator 0.0 0.0 _skyboxangle) false false)
  (Rendering|Components|Light|SetIntensity (Variables|Default|GetRectLight) (Variables|Default|GetBrightness)))

(fn ConstructionScript
  (bind _skyboxangle (Variables|Default|GetSkyBoxAngle))
  (Components|InstancedStaticMesh|AddInstance (Variables|Default|GetSkyBox) (Math|Transform|MakeTransform "0, 0, 0" "0.000000,0.000000,180.000000" "1.000000,1.000000,1.000000") false)
  (Components|InstancedStaticMesh|AddInstance (Variables|Default|GetLeg1) (Math|Transform|MakeTransform "0, 0, 0" "0.000000,0.000000,-110.000000" "1.000000,1.000000,1.000000") false)
  (Components|InstancedStaticMesh|AddInstance (Variables|Default|GetLeg2) (Math|Transform|MakeTransform "0, 0, 0" "0.000000,0.000000,-90.000000" "1.000000,1.000000,1.000000") false)
  (Transformation|AddLocalRotation (Variables|Default|GetRectLight) (Math|Rotator|MakeRotator 0.0 0.0 _skyboxangle) false false)
  (Components|InstancedStaticMesh|UpdateInstanceTransform (Variables|Default|GetSkyBox) 0 (Math|Transform|MakeTransform "0, 0, 0" (Math|Rotator|MakeRotator _skyboxangle 0.0 0.0) "1.000000,1.000000,1.000000") false false false)
  (Rendering|Components|Light|SetIntensity (Variables|Default|GetRectLight) (Variables|Default|GetBrightness))
  (Rendering|Components|Light|SetLightColor (Variables|Default|GetRectLight) (Variables|Default|GetSkyboxColor) true))